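; Demo loot actor for the Loot and Pickup VFX pack showroom, pairing a loot mesh with light pillar and glow Niagara effects.
; The Construction Script applies the configurable Niagara systems and mesh material, then feeds VFXBPScaling into each effect's UserScale parameter.
; UpdateVFX, marked as a disposable showcase utility, reapplies the systems and material, resetting parameter overrides without setting the scale again.
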(event Custom|Update%20VFX
  ;[1 1 1] Showcase utility - Free to delete after
  (Class|NiagaraComponent|SetAsset (Variables|Default|GetNS_LightPillarVFX) (Variables|VFX|GetUserNS_LightPillar) true)
  (Class|NiagaraComponent|SetAsset (Variables|Default|GetNS_GlowVFX) (Variables|VFX|GetUserNS_Glow) true)
  (Rendering|Material|SetMaterial (Variables|Default|GetSM_Loot) 0 (Variables|VFX|GetSphere%20Material)))

(event EventBeginPlay)

(event Collision|EventActorBeginOverlap
  (params (OtherActor :type Actor%20Object%20Reference)))

(event EventTick
  (params (DeltaSeconds :type Float%20%28single-precision%29)))

(fn ConstructionScript
  (bind _vfxbpscaling (Variables|Default|GetVFXBPScaling))
  (bind _ns_lightpillarvfx (Variables|Default|GetNS_LightPillarVFX))
  (bind _ns_glowvfx (Variables|Default|GetNS_GlowVFX))
  (Class|NiagaraComponent|SetAsset _ns_lightpillarvfx (Variables|VFX|GetUserNS_LightPillar) true)
  (Class|NiagaraComponent|SetAsset _ns_glowvfx (Variables|VFX|GetUserNS_Glow) true)
  (Rendering|Material|SetMaterial (Variables|Default|GetSM_Loot) 0 (Variables|VFX|GetSphere%20Material))
  (Niagara|SetNiagaraVariable(Float) _ns_lightpillarvfx "UserScale" _vfxbpscaling)
  (Niagara|SetNiagaraVariable(Float) _ns_glowvfx "UserScale" _vfxbpscaling))