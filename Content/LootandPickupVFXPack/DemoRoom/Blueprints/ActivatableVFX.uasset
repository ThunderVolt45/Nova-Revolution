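; Demo room actor for the loot and pickup VFX pack that plays a configurable Niagara effect, switched on and off externally.
; The construction script assigns the chosen VFX asset to the Niagara component, and ToggleActivation stores the passed-in button state.
; Tick runs through a Delay, so at that interval it restarts the effect with a reset while the state is on, or deactivates it otherwise.
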(event Custom|ToggleActivation
  (params (State :type Boolean))
  (Variables|Default|SetButtonState State))

(event EventBeginPlay)

(event Collision|EventActorBeginOverlap
  (params (OtherActor :type Actor%20Object%20Reference)))

(event EventTick
  (params (DeltaSeconds :type Float%20%28single-precision%29))
  (bind _ns_lootspawn (Variables|Default|GetNS_LootSpawn))
  (Utilities|FlowControl|Delay (Variables|Default|GetDelay))
  (if (Variables|Default|GetButtonState)
    (Components|Activation|SetActive _ns_lootspawn true true)
    (else
      (Components|Activation|Deactivate _ns_lootspawn))))

(fn ConstructionScript
  (Class|NiagaraComponent|SetAsset (Variables|Default|GetNS_LootSpawn) (Variables|Default|GetVFX) true))